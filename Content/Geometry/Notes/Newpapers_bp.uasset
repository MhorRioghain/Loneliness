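; Interactable newspaper prop that the player can read as an on-screen image.
; The trigger volume enables input and shows a hint on overlap; Interactions toggles between hiding the mesh with ReadNews and restoring it with EndReadNews.
; Leaving the volume disables input, clears the hint and closes the reading view.
; The construction script uses NewsNumber to pick one of four material and widget-image pairs.
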(event `self.TriggerVolume.OnComponentBeginOverlap`
  (params (OverlappedComponent :type "PrimitiveComponent Object Reference") (OtherActor :type "Actor Object Reference") (OtherComp :type "PrimitiveComponent Object Reference") (OtherBodyIndex :type Integer) (bFromSweep :type Boolean) (SweepResult :type "HitResult Structure (by ref)"))
  ;[1 1 1] Newspaper Input
  (`self.EnableInput` (`GameplayStatics.GetPlayerController` 0))
  (bind _returntipsreference (`/Game/FirstPerson/Blueprints/ShowWidgets_F.ShowHint` (`self.HintKeyText`) (`self.HintColor`) (`self.TipsReference`)))
  (set `self.TipsReference` _returntipsreference))

(event `InputAction|Interactions`
  (params (Key :type "Key Structure" :default "AnyKey"))
  (bind _newspaper (`self.newspaper`))
  (bind _readnewsreference (`self.ReadNewsReference`))
  ;[1 1 1] Read newspaper
  (:`Pressed`
    (if (`self.IsRead?`)
      (set `self.IsRead?` false)
      (`SceneComponent.SetHiddenInGame` _newspaper true false)
      (bind _returnreadnewsreferencce (`/Game/FirstPerson/Blueprints/ShowWidgets_F.ReadNews` (`self.WidgetImage`) (`self.TipsReference`) _readnewsreference))
      (set `self.ReadNewsReference` _returnreadnewsreferencce)
      (else
        (set `self.IsRead?` true)
        (`SceneComponent.SetHiddenInGame` _newspaper false false :!label _label)
        (`/Game/FirstPerson/Blueprints/ShowWidgets_F.EndReadNews` _readnewsreference)))))

(event `self.TriggerVolume.OnComponentEndOverlap`
  (params (OverlappedComponent :type "PrimitiveComponent Object Reference") (OtherActor :type "Actor Object Reference") (OtherComp :type "PrimitiveComponent Object Reference") (OtherBodyIndex :type Integer))
  ;[1 1 1] Newspaper Input
  (`self.DisableInput` (`GameplayStatics.GetPlayerController` 0))
  (`/Game/FirstPerson/Blueprints/ShowWidgets_F.HideHint` (`self.TipsReference`))
  ;[1 1 1] Read newspaper
  (set `self.IsRead?` true)
  (goto _label))

(fn `UserConstructionScript`
  (bind _newsnumber (`self.NewsNumber`))
  (`PrimitiveComponent.SetMaterial` (`self.newspaper`) 0 (select `/Game/Geometry/Notes/ENewsNumber` _newsnumber :`NewEnumerator0` "/Game/Geometry/Notes/News1.News1" :`NewEnumerator1` "/Game/Geometry/Notes/News2.News2" :`NewEnumerator2` "/Game/Geometry/Notes/News3.News3" :`NewEnumerator3` "/Game/Geometry/Notes/News4.News4" :!type "MaterialInterface Object Reference"))
  (set `self.WidgetImage` (select `/Game/Geometry/Notes/ENewsNumber` _newsnumber :`NewEnumerator0` "/Game/Geometry/Notes/newspaper1.newspaper1" :`NewEnumerator1` "/Game/Geometry/Notes/newspaper2.newspaper2" :`NewEnumerator2` "/Game/Geometry/Notes/newspaper3.newspaper3" :`NewEnumerator3` "/Game/Geometry/Notes/newspaper4.newspaper4" :!type "Texture2D Object Reference"))
  (set `self.HintColor` (struct :`R` 0.06301 :`G` 0.036889 :`B` 0.584079 :`A` 1.0)))