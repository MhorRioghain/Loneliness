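; DrinkMe is a pickup actor that grants the first-person character superhuman power.
; Entering its trigger enables input on the actor and shows a colored "Drink me" hint, hidden after a short delay or on leaving.
; Pressing the Interactions action while input is enabled sets the power flag on the overlapping character and destroys the pickup.
; Leaving the trigger disables input again.
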(event `InputAction|Interactions`
  (params (Key :type "Key Structure" :default "AnyKey"))
  ;[1 1 1] Enable Super human powers
  (:`Pressed`
    (bind _asfirst_person_character (cast `/Game/FirstPerson/Blueprints/FirstPersonCharacter` (stale `self.Trigger.OnComponentBeginOverlap` OtherActor)))
    (set `/Game/FirstPerson/Blueprints/FirstPersonCharacter.HaveSuperHumanPower?` true _asfirst_person_character)
    (`self.K2_DestroyActor`)))

(event `self.Trigger.OnComponentBeginOverlap`
  (params (OverlappedComponent :type "PrimitiveComponent Object Reference") (OtherActor :type "Actor Object Reference") (OtherComp :type "PrimitiveComponent Object Reference") (OtherBodyIndex :type Integer) (bFromSweep :type Boolean) (SweepResult :type "HitResult Structure (by ref)"))
  (bind _tips_reference (`self.Tips Reference`))
  ;[1 1 1] Enable/Disable Input
  (`self.EnableInput` (`GameplayStatics.GetPlayerController` 0))
  (bind _returntipsreference (`/Game/FirstPerson/Blueprints/ShowWidgets_F.ShowHint` "Drink me" (`self.Color`) _tips_reference))
  (set `self.Tips Reference` _returntipsreference)
  (`KismetSystemLibrary.Delay` 2.0)
  (`/Game/FirstPerson/Blueprints/ShowWidgets_F.HideHint` _tips_reference :!label _label))

(event `self.Trigger.OnComponentEndOverlap`
  (params (OverlappedComponent :type "PrimitiveComponent Object Reference") (OtherActor :type "Actor Object Reference") (OtherComp :type "PrimitiveComponent Object Reference") (OtherBodyIndex :type Integer))
  ;[1 1 1] Enable/Disable Input
  (`self.DisableInput` (`GameplayStatics.GetPlayerController` 0))
  (goto _label))

(fn `UserConstructionScript`
  (set `self.Color` (struct :`R` 0.06301 :`G` 0.036889 :`B` 0.584079 :`A` 1.0)))