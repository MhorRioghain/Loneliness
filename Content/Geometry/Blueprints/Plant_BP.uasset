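; Plant Blueprint that procedurally builds a row of randomly sized static mesh plants.
; The Construction Script adds HowManyPlants mesh components, placing each along local X by a random unit vector's X scaled by Modifier, at a fixed height.
; Width and height scale vary randomly per plant, while depth stays constant.
; The Event Graph holds only disabled stubs, so it has no runtime logic.
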(fn `UserConstructionScript`
  (for _ (range 1 (+ (`self.HowManyPlants?`) 1))
    (`AddComponent|Static Mesh Component_0` :`RelativeTransform` (`KismetMathLibrary.MakeTransform` (`KismetMathLibrary.MakeVector` (.x (* (`KismetMathLibrary.RandomUnitVector`) (`self.Modifier`))) 0.0 250.0) (struct) (`KismetMathLibrary.MakeVector` (`KismetMathLibrary.RandomFloatInRange` 1.0 3.5) 1.0 (`KismetMathLibrary.RandomFloatInRange` 1.0 3.0))))))