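; Level exit door that ends the level when the first-person player holds the key type it requires.
; Its trigger volume toggles input and the interaction hint; Interactions searches OwnedKeys, playing a locked sound with a key-color hint if none match.
; A match shows the LevelComplete widget with the newspapers-read count, then opens the "start" level after a delay.
; The construction script derives door material, hint text and hint color from the required key type.
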(event `self.TriggerVolume.OnComponentBeginOverlap`
  (params (OverlappedComponent :type "PrimitiveComponent Object Reference") (OtherActor :type "Actor Object Reference") (OtherComp :type "PrimitiveComponent Object Reference") (OtherBodyIndex :type Integer) (bFromSweep :type Boolean) (SweepResult :type "HitResult Structure (by ref)"))
  ;[1 1 1] Door Input and Input Tips
  (`self.EnableInput` (`GameplayStatics.GetPlayerController` 0))
  (bind _returntipsreference (`/Game/FirstPerson/Blueprints/ShowWidgets_F.ShowHint` (`self.HintKeyText`) (`self.HintKeyColor`) (`self.TipsReference`)))
  (set `self.TipsReference` _returntipsreference))

(event `InputAction|Interactions`
  (params (Key :type "Key Structure" :default "AnyKey"))
  ;[1 1 1] Door Open/Close and show Tips
  (:`Pressed`
    (bind _asfirst_person_character (cast `/Game/FirstPerson/Blueprints/FirstPersonCharacter` (stale `self.TriggerVolume.OnComponentBeginOverlap` OtherActor)))
    (bind _ownedkeys (`/Game/FirstPerson/Blueprints/FirstPersonCharacter.OwnedKeys` _asfirst_person_character))
    (for _array_element _ownedkeys
      (if (`|EnumEquality` _array_element (`self.RequeredKeyType`))
        (set `self.HaveKey?` true)
        (bind _returnvalue (`|CreateWidget` "/Game/FirstPerson/Blueprints/LevelComplete.LevelComplete_C"))
        (set `/Game/FirstPerson/Blueprints/LevelComplete.NewsCount` (`KismetTextLibrary.Conv_IntToText` (`/Game/FirstPerson/Blueprints/FirstPersonCharacter.NewspapersRead` _asfirst_person_character)) _returnvalue)
        (`UserWidget.AddToViewport` _returnvalue 0)
        (`WidgetBlueprintLibrary.SetInputMode_UIOnlyEx` (`GameplayStatics.GetPlayerController` 0) _returnvalue "LockOnCapture")
        (`KismetSystemLibrary.Delay` 5.0)
        (`GameplayStatics.OpenLevel` "start")))
    (if (== (`KismetArrayLibrary.Array_Length` _ownedkeys) 0)
      (`GameplayStatics.PlaySoundAtLocation` "/Game/Audio/default_locked.default_locked" (`self.K2_GetActorLocation`) :!label _label)
      (bind _returntipsreference (`/Game/FirstPerson/Blueprints/ShowWidgets_F.ShowHint` (`self.HintText`) (`self.HintColor`) (`self.TipsReference`)))
      (set `self.TipsReference` _returntipsreference)
      (elif (not (`self.HaveKey?`))
        (goto _label)))))

(event `self.TriggerVolume.OnComponentEndOverlap`
  (params (OverlappedComponent :type "PrimitiveComponent Object Reference") (OtherActor :type "Actor Object Reference") (OtherComp :type "PrimitiveComponent Object Reference") (OtherBodyIndex :type Integer))
  ;[1 1 1] Door Input and Input Tips
  (`self.DisableInput` (`GameplayStatics.GetPlayerController` 0))
  (`/Game/FirstPerson/Blueprints/ShowWidgets_F.HideHint` (`self.TipsReference`)))

(fn `UserConstructionScript`
  (bind _requeredkeytype (`self.RequeredKeyType`))
  (`PrimitiveComponent.SetMaterial` (`self.door`) 1 (select `/Game/Geometry/Blueprints/EKeyType` _requeredkeytype :`NewEnumerator0` "/Game/Geometry/Materials/metal.metal" :`NewEnumerator1` "/Game/Geometry/Materials/metal_blue.metal_blue" :`NewEnumerator2` "/Game/Geometry/Materials/metal_green.metal_green" :`NewEnumerator3` "/Game/Geometry/Materials/metal_red.metal_red" :!type "MaterialInterface Object Reference"))
  (set `self.HintText` (select `/Game/Geometry/Blueprints/EKeyType` _requeredkeytype :`NewEnumerator1` "You need a BLUE key " :`NewEnumerator2` "You need a GREEN key" :`NewEnumerator3` "You need a RED key" :!type "Text"))
  (set `self.HintColor` (select `/Game/Geometry/Blueprints/EKeyType` _requeredkeytype :`NewEnumerator1` (struct :`G` 0.26649 :`B` 0.965 :`A` 1.0) :`NewEnumerator2` (struct :`G` 0.8 :`B` 0.075686 :`A` 1.0) :`NewEnumerator3` (struct :`R` 0.815 :`G` 0.0326 :`B` 0.039924 :`A` 1.0) :!type "LinearColor Structure"))
  (set `self.HintKeyColor` (struct :`R` 0.23074 :`G` 0.130136 :`B` 0.806952 :`A` 1.0)))