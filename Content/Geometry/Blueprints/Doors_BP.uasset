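; Interactive door that swings open and shut on the Interactions input and streams the levels on either side.
; A trigger box enables input and briefly shows a key hint, while a rotation timeline drives the door and auto-closes it after a delay.
; Two volumes each load their side's level, unloading it on exit unless the opposite volume was entered last, with a delay if the door is open.
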(event `self.TriggerBox.OnComponentBeginOverlap`
  (params (OverlappedComponent :type "PrimitiveComponent Object Reference") (OtherActor :type "Actor Object Reference") (OtherComp :type "PrimitiveComponent Object Reference") (OtherBodyIndex :type Integer) (bFromSweep :type Boolean) (SweepResult :type "HitResult Structure (by ref)"))
  (bind _tipsreference (`self.TipsReference`))
  ;[1 1 1] Door Input and Output Tips
  (`self.EnableInput` (`GameplayStatics.GetPlayerController` 0))
  (bind _returntipsreference (`/Game/FirstPerson/Blueprints/ShowWidgets_F.ShowHint` (`self.HintKeyText`) (`self.HintColor`) _tipsreference))
  (set `self.TipsReference` _returntipsreference)
  (`KismetSystemLibrary.Delay` 2.0)
  (`/Game/FirstPerson/Blueprints/ShowWidgets_F.HideHint` _tipsreference :!label _label))

(event `InputAction|Interactions`
  (params (Key :type "Key Structure" :default "AnyKey"))
  ;[1 1 1] Door Open/Close
  (:`Pressed`
    (bind _asfirst_person_character (cast `/Game/FirstPerson/Blueprints/FirstPersonCharacter` (stale `self.TriggerBox.OnComponentBeginOverlap` OtherActor)))
    (`GameplayStatics.PlaySoundAtLocation` "/Game/Audio/default_move.default_move" (`self.K2_GetActorLocation` _asfirst_person_character))
    (if (`self.IsOpen?`)
      (set `self.IsOpen?` false :!label _label_2)
      (bind (_direction _driver) (`Timeline|Door Timeline` :!via `Reverse` :!label _label_3)
        (:`Update`
          (set `self.IsAnimDone?` false)
          (`SceneComponent.K2_SetRelativeRotation` (`self.door`) (`KismetMathLibrary.RLerp` (`self.DoorStart`) (`self.DoorEnd`) _driver) false false))
        (:`Finished`
          (set `self.IsAnimDone?` true)
          (`KismetSystemLibrary.Delay` 5.0)
          (if (`self.IsOpen?`)
            (if (`self.IsAnimDone?`)
              (goto _label_2)))))
      (else
        (set `self.IsOpen?` true)
        (goto _label_3)))))

(event `self.TriggerBox.OnComponentEndOverlap`
  (params (OverlappedComponent :type "PrimitiveComponent Object Reference") (OtherActor :type "Actor Object Reference") (OtherComp :type "PrimitiveComponent Object Reference") (OtherBodyIndex :type Integer))
  ;[1 1 1] Door Input and Output Tips
  (`self.DisableInput` (`GameplayStatics.GetPlayerController` 0))
  (goto _label))

(event `self.LvlBox1.OnComponentBeginOverlap`
  (params (OverlappedComponent :type "PrimitiveComponent Object Reference") (OtherActor :type "Actor Object Reference") (OtherComp :type "PrimitiveComponent Object Reference") (OtherBodyIndex :type Integer) (bFromSweep :type Boolean) (SweepResult :type "HitResult Structure (by ref)"))
  ;[1 1 1] Level Streaming
  (set `self.OutsideRoom?` true)
  (set `self.InsideRoom?` false)
  (`GameplayStatics.LoadStreamLevel` (`self.LevelLeft`) true))

(event `self.LvlBox1.OnComponentEndOverlap`
  (params (OverlappedComponent :type "PrimitiveComponent Object Reference") (OtherActor :type "Actor Object Reference") (OtherComp :type "PrimitiveComponent Object Reference") (OtherBodyIndex :type Integer))
  ;[1 1 1] Level Streaming
  (if (`self.IsOpen?`)
    (`KismetSystemLibrary.Delay` 7.0))
  (if (not (`self.InsideRoom?`))
    (`GameplayStatics.UnloadStreamLevel` (`self.LevelLeft`))))

(event `self.LvlBox2.OnComponentBeginOverlap`
  (params (OverlappedComponent :type "PrimitiveComponent Object Reference") (OtherActor :type "Actor Object Reference") (OtherComp :type "PrimitiveComponent Object Reference") (OtherBodyIndex :type Integer) (bFromSweep :type Boolean) (SweepResult :type "HitResult Structure (by ref)"))
  ;[1 1 1] Level Streaming
  (set `self.InsideRoom?` true)
  (set `self.OutsideRoom?` false)
  (`GameplayStatics.LoadStreamLevel` (`self.LevelRight`) true))

(event `self.LvlBox2.OnComponentEndOverlap`
  (params (OverlappedComponent :type "PrimitiveComponent Object Reference") (OtherActor :type "Actor Object Reference") (OtherComp :type "PrimitiveComponent Object Reference") (OtherBodyIndex :type Integer))
  ;[1 1 1] Level Streaming
  (if (`self.IsOpen?`)
    (`KismetSystemLibrary.Delay` 7.0))
  (if (not (`self.OutsideRoom?`))
    (`GameplayStatics.UnloadStreamLevel` (`self.LevelRight`))))

(fn `UserConstructionScript`
  (set `self.HintColor` (struct :`R` 0.06301 :`G` 0.036889 :`B` 0.584079 :`A` 1.0)))