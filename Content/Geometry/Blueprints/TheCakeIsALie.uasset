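; TheCakeIsALie is an "Eat me" pickup that grants the player's FirstPersonCharacter the size-shifting ability.
; Entering its trigger enables input and shows a hint tinted by the construction script's color, hidden after two seconds or on exit.
; Exit also disables input.
; Pressing Interactions casts the overlap's OtherActor to the character, sets HaveSizeShifting and destroys the pickup.
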(event `InputAction|Interactions`
  (params (Key :type "Key Structure" :default "AnyKey"))
  (:`Pressed`
    (bind _asfirst_person_character (cast `/Game/FirstPerson/Blueprints/FirstPersonCharacter` (stale `self.Trigger.OnComponentBeginOverlap` OtherActor)))
    (set `/Game/FirstPerson/Blueprints/FirstPersonCharacter.HaveSizeShifting?` true _asfirst_person_character)
    (`self.K2_DestroyActor`)))

(event `self.Trigger.OnComponentBeginOverlap`
  (params (OverlappedComponent :type "PrimitiveComponent Object Reference") (OtherActor :type "Actor Object Reference") (OtherComp :type "PrimitiveComponent Object Reference") (OtherBodyIndex :type Integer) (bFromSweep :type Boolean) (SweepResult :type "HitResult Structure (by ref)"))
  (bind _tipsreference (`self.TipsReference`))
  (`self.EnableInput` (`GameplayStatics.GetPlayerController` 0))
  (bind _returntipsreference (`/Game/FirstPerson/Blueprints/ShowWidgets_F.ShowHint` "Eat me" (`self.Color`) _tipsreference))
  (set `self.TipsReference` _returntipsreference)
  (`KismetSystemLibrary.Delay` 2.0)
  (`/Game/FirstPerson/Blueprints/ShowWidgets_F.HideHint` _tipsreference :!label _label))

(event `self.Trigger.OnComponentEndOverlap`
  (params (OverlappedComponent :type "PrimitiveComponent Object Reference") (OtherActor :type "Actor Object Reference") (OtherComp :type "PrimitiveComponent Object Reference") (OtherBodyIndex :type Integer))
  (`self.DisableInput` (`GameplayStatics.GetPlayerController` 0))
  (goto _label))

(fn `UserConstructionScript`
  (set `self.Color` (struct :`R` 0.06301 :`G` 0.036889 :`B` 0.584079 :`A` 1.0)))