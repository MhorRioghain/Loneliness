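; Dynamic wall that slides aside and streams levels in and out as either of its two trigger volumes is overlapped.
; Entering a trigger records the side, starts loading its left or right level without blocking, and plays a timeline lerping Wall2's relative location.
; Leaving waits briefly if the animation is unfinished, then unloads that level and reverses the wall unless the other trigger was entered last.
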(fn `UserConstructionScript`)