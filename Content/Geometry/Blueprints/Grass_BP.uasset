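; Grass Blueprint that scatters a patch of static mesh components around the actor, presumably grass meshes.
; The construction script adds HowManyGrass components at flat positions taken from random unit vectors scaled by Modifier.
; Each gets a random yaw and slight random per-axis scale, with no seeded stream, so the layout changes whenever construction reruns.
; The event graph holds no active logic.
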(fn `UserConstructionScript`
  (bind _returnvalue (`KismetMathLibrary.RandomFloatInRange` 0.7 1.3))
  (for _ (range 1 (+ (`self.HowManyGrass?`) 1))
    (`AddComponent|Static Mesh Component_0` :`RelativeTransform` (`KismetMathLibrary.MakeTransform` (`KismetMathLibrary.MakeVector` (.x (* (`KismetMathLibrary.RandomUnitVector`) (`self.Modifier`))) (.y (* (`KismetMathLibrary.RandomUnitVector`) (`self.Modifier`)))) (`KismetMathLibrary.MakeRotator` 0.0 0.0 (`KismetMathLibrary.RandomFloatInRange` 0.0 180.0)) (`KismetMathLibrary.MakeVector` _returnvalue _returnvalue (`KismetMathLibrary.RandomFloatInRange` 0.7 1.3))))))