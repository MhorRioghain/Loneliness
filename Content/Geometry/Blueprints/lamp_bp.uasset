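; Lamp Blueprint with a point light whose color is picked from a LightColor option and can be switched on or off.
; The construction script applies the chosen color and calls TurnLight, which sets a per-color intensity or zero based on IsLightsOn.
; The SuperAbilities event flips IsLightsOn through a FlipFlop and reapplies TurnLight.
; An older color-comparison intensity branch is left unconnected.
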(event `self.ReceiveBeginPlay`)

(event `/Game/FirstPerson/Blueprints/SuperPowers.SuperAbilities`
  (`/Engine/EditorBlueprintResources/StandardMacros.FlipFlop`
    (:`A`
      (set `self.Is Lights On?` false))
    (:`B`
      (set `self.Is Lights On?` true)))
  (`self.TurnLight` (`self.Is Lights On?`)))

(fn `TurnLight`
  (params (`IsLightOn?` :type Boolean))
  (bind _pointlight (`self.PointLight`))
  (if `IsLightOn?`
    (`LightComponent.SetIntensity` _pointlight (select `/Game/Geometry/Blueprints/ELampColor` (`self.LightColor`) :`NewEnumerator0` 1500.0 :`NewEnumerator1` 4000.0 :`NewEnumerator2` 1500.0 :`NewEnumerator3` 4000.0 :`NewEnumerator4` 3000.0 :!type "Float (single-precision)"))
    (else
      (`LightComponent.SetIntensity` _pointlight 0.0))))

(fn `UserConstructionScript`
  (`LightComponent.SetLightColor` (`self.PointLight`) (select `/Game/Geometry/Blueprints/ELampColor` (`self.LightColor`) :`NewEnumerator0` (struct :`R` 1.0 :`G` 1.0 :`B` 1.0 :`A` 1.0) :`NewEnumerator1` (struct :`R` 1.0 :`A` 1.0) :`NewEnumerator2` (struct :`R` 1.0 :`G` 1.0 :`A` 1.0) :`NewEnumerator3` (struct :`G` 0.7 :`B` 1.0 :`A` 1.0) :`NewEnumerator4` (struct :`G` 1.0 :`A` 1.0) :!type "LinearColor Structure") true)
  (`self.TurnLight` (`self.Is Lights On?`)))