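; RandomPapers is a prop Blueprint that scatters paper static meshes flat around its origin as set dressing.
; The construction script loops HowManyPapers times, randomly picking one of two AddStaticMeshComponent nodes.
; Each mesh gets a random yaw and an XY offset from random unit vectors scaled by Modifier.
; Randomness is unseeded, so the layout reshuffles whenever construction reruns, and the event graph holds only disabled stubs.
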(fn `UserConstructionScript`
  (bind _returnvalue (`KismetMathLibrary.MakeTransform` (`KismetMathLibrary.MakeVector` (.x (* (`KismetMathLibrary.RandomUnitVector`) (`self.Modifier`))) (.y (* (`KismetMathLibrary.RandomUnitVector`) (`self.Modifier`)))) (`KismetMathLibrary.MakeRotator` 0.0 0.0 (`KismetMathLibrary.RandomFloatInRange` 0.0 360.0))))
  (for _ (range 1 (+ (`self.HowManyPapers?`) 1))
    (if (`KismetMathLibrary.RandomBool`)
      (`AddComponent|Static Mesh Component_0` :`RelativeTransform` _returnvalue)
      (else
        (`AddComponent|Static Mesh Component_1` :`RelativeTransform` _returnvalue)))))