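; Interactive door Blueprint that the player can swing open and closed while inside its trigger box.
; Overlapping the trigger enables input and shows a colored key hint, and leaving disables input and hides it.
; The Interactions action plays a sound at the FirstPersonCharacter's location, then a FlipFlop alternately plays or reverses a Timeline that lerps the door's relative rotation between start and end.
; The Construction Script sets the hint color.
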(event `self.TriggerBox.OnComponentBeginOverlap`
  (params (OverlappedComponent :type "PrimitiveComponent Object Reference") (OtherActor :type "Actor Object Reference") (OtherComp :type "PrimitiveComponent Object Reference") (OtherBodyIndex :type Integer) (bFromSweep :type Boolean) (SweepResult :type "HitResult Structure (by ref)"))
  ;[1 1 1] Door Input and Input Tips
  (`self.EnableInput` (`GameplayStatics.GetPlayerController` 0))
  (bind _returntipsreference (`/Game/FirstPerson/Blueprints/ShowWidgets_F.ShowHint` (`self.HintKeyText`) (`self.HintColor`) (`self.TipsReference`)))
  (set `self.TipsReference` _returntipsreference))

(event `InputAction|Interactions`
  (params (Key :type "Key Structure" :default "AnyKey"))
  ;[1 1 1] Door Open/Close and show Tips
  (:`Pressed`
    (bind _asfirst_person_character (cast `/Game/FirstPerson/Blueprints/FirstPersonCharacter` (stale `self.TriggerBox.OnComponentBeginOverlap` OtherActor)))
    (`GameplayStatics.PlaySoundAtLocation` "/Game/Audio/default_move.default_move" (`self.K2_GetActorLocation` _asfirst_person_character)) ; Play teleportation sound
    (`/Engine/EditorBlueprintResources/StandardMacros.FlipFlop`
      (:`A`
        (bind (_direction _driver) (`Timeline|Door Timeline` :!label _label)
          (:`Update`
            (`SceneComponent.K2_SetRelativeRotation` (`self.door`) (`KismetMathLibrary.RLerp` (`self.DoorStart`) (`self.DoorEnd`) _driver) false false))))
      (:`B`
        (goto _label :!via `Reverse`)))))

(event `self.TriggerBox.OnComponentEndOverlap`
  (params (OverlappedComponent :type "PrimitiveComponent Object Reference") (OtherActor :type "Actor Object Reference") (OtherComp :type "PrimitiveComponent Object Reference") (OtherBodyIndex :type Integer))
  ;[1 1 1] Door Input and Input Tips
  (`self.DisableInput` (`GameplayStatics.GetPlayerController` 0))
  (`/Game/FirstPerson/Blueprints/ShowWidgets_F.HideHint` (`self.TipsReference`)))

(fn `UserConstructionScript`
  (set `self.HintColor` (struct :`R` 0.06301 :`G` 0.036889 :`B` 0.584079 :`A` 1.0)))