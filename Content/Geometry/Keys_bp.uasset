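; Collectible colored key pickup that adds its key type to the first-person character's owned keys.
; The construction script sets the key's material, pickup message and hint color from KeyType.
; Entering the trigger volume enables input and shows a key hint; leaving disables input and hides it.
; Pressing Interactions records the key, plays a portal sound, shows the found-key message for a second, then destroys the actor.
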(event `self.TriggerVolume.OnComponentBeginOverlap`
  (params (OverlappedComponent :type "PrimitiveComponent Object Reference") (OtherActor :type "Actor Object Reference") (OtherComp :type "PrimitiveComponent Object Reference") (OtherBodyIndex :type Integer) (bFromSweep :type Boolean) (SweepResult :type "HitResult Structure (by ref)"))
  ;[1 1 1] Key Input and Input Tips
  (`self.EnableInput` (`GameplayStatics.GetPlayerController` 0))
  (bind _returntipsreference (`/Game/FirstPerson/Blueprints/ShowWidgets_F.ShowHint` (`self.HintKeyText`) (`self.HintColor`) (`self.TipsReference`)))
  (set `self.TipsReference` _returntipsreference))

(event `InputAction|Interactions`
  (params (Key :type "Key Structure" :default "AnyKey"))
  ;[1 1 1] Get Key and show Tips
  (:`Pressed`
    (bind _asfirst_person_character (cast `/Game/FirstPerson/Blueprints/FirstPersonCharacter` (stale `self.TriggerVolume.OnComponentBeginOverlap` OtherActor)))
    (`KismetArrayLibrary.Array_Add` (`/Game/FirstPerson/Blueprints/FirstPersonCharacter.OwnedKeys` _asfirst_person_character) (`self.KeyType`))
    (`GameplayStatics.PlaySoundAtLocation` "/Game/Audio/portal_enter1.portal_enter1" (`self.K2_GetActorLocation`)) ; Play teleportation sound
    (bind _returntipsreference (`/Game/FirstPerson/Blueprints/ShowWidgets_F.ShowHint` (`self.HintText`) (`self.HintColor`) (`self.TipsReference`)))
    (`KismetSystemLibrary.Delay` 1.0)
    (`/Game/FirstPerson/Blueprints/ShowWidgets_F.HideHint` _returntipsreference)
    (`self.K2_DestroyActor`)))

(event `self.TriggerVolume.OnComponentEndOverlap`
  (params (OverlappedComponent :type "PrimitiveComponent Object Reference") (OtherActor :type "Actor Object Reference") (OtherComp :type "PrimitiveComponent Object Reference") (OtherBodyIndex :type Integer))
  ;[1 1 1] Key Input and Input Tips
  (`self.DisableInput` (`GameplayStatics.GetPlayerController` 0))
  (`/Game/FirstPerson/Blueprints/ShowWidgets_F.HideHint` (`self.TipsReference`)))

(fn `UserConstructionScript`
  (bind _keytype (`self.KeyType`))
  (`PrimitiveComponent.SetMaterial` (`self.key`) 0 (select `/Game/Geometry/EKeyType` _keytype :`NewEnumerator0` "/Game/Geometry/Materials/key.key" :`NewEnumerator1` "/Game/Geometry/Materials/key_blue.key_blue" :`NewEnumerator2` "/Game/Geometry/Materials/key_green.key_green" :`NewEnumerator3` "/Game/Geometry/Materials/key_red.key_red" :!type "MaterialInterface Object Reference"))
  (set `self.HintText` (select `/Game/Geometry/EKeyType` _keytype :`NewEnumerator1` "You found the BLUE key " :`NewEnumerator2` "You found the GREEN key" :`NewEnumerator3` "You found the RED key" :!type "Text"))
  (set `self.HintColor` (select `/Game/Geometry/EKeyType` _keytype :`NewEnumerator1` (struct :`G` 0.26649 :`B` 0.965 :`A` 1.0) :`NewEnumerator2` (struct :`G` 0.8 :`B` 0.075686 :`A` 1.0) :`NewEnumerator3` (struct :`R` 0.815 :`G` 0.0326 :`B` 0.039924 :`A` 1.0) :!type "LinearColor Structure")))