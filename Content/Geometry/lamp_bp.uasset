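; Lamp Blueprint whose point light takes one of five preset colors: white, red, yellow, blue or green.
; The construction script uses the LightColor selection to set both the light's color and a matching intensity.
; The event graph has no active logic, only empty events and an unreachable color-based intensity chain.
; That chain calls ColorCompare, whose RGB equality check is left unconnected.
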(event `self.ReceiveBeginPlay`)

(fn `UserConstructionScript`
  (bind _pointlight (`self.PointLight`))
  (bind _lightcolor (`self.LightColor`))
  (`LightComponent.SetLightColor` _pointlight (select `/Game/Geometry/ELampColor` _lightcolor :`NewEnumerator0` (struct :`R` 1.0 :`G` 1.0 :`B` 1.0 :`A` 1.0) :`NewEnumerator1` (struct :`R` 1.0 :`A` 1.0) :`NewEnumerator2` (struct :`R` 1.0 :`G` 1.0 :`A` 1.0) :`NewEnumerator3` (struct :`G` 0.7 :`B` 1.0 :`A` 1.0) :`NewEnumerator4` (struct :`G` 1.0 :`A` 1.0) :!type "LinearColor Structure") true)
  (`LightComponent.SetIntensity` _pointlight (select `/Game/Geometry/ELampColor` _lightcolor :`NewEnumerator0` 1500.0 :`NewEnumerator1` 4000.0 :`NewEnumerator2` 1500.0 :`NewEnumerator3` 4000.0 :`NewEnumerator4` 3000.0 :!type "Float (single-precision)")))